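; SRCubeBP is a cube Blueprint in test content that displays a symbol texture on its static mesh.
; SetSymbol stores the ID and picks a texture from a fixed set, with -1 showing the SR logo, then passes it to SetTexture.
; SetTexture writes the material's Texture parameter, lazily creating a dynamic material instance on slot 0 and retrying when none exists.
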(event Custom|SetTexture
  (params (InTexture :type Texture%202D%20Object%20Reference))
  (bind _staticmesh (Variables|Default|GetStaticMesh))
  (bind _asmaterial_instance_dynamic (Utilities|Casting|CastToMaterialInstanceDynamic (Rendering|Material|GetMaterial _staticmesh 0) :!label _label)
    (:then
      (Rendering|Material|SetTextureParameterValue _asmaterial_instance_dynamic "Texture" InTexture))
    (:CastFailed
      (Rendering|Material|CreateDynamicMaterialInstance _staticmesh 0 0 "None" :!class /Script/Engine.PrimitiveComponent)
      (goto _label))))

(event Custom|SetSymbol
  (params (SymbolId :type Integer))
  (Variables|Default|SetSymbolID SymbolId)
  (CallFunction|SetTexture (select (== SymbolId -1) "/SymbolRecognizerPlugin/Resources/TestContent/Textures/T_SRLogo512.T_SRLogo512" (Utilities|Select :Index (Variables|Default|GetSymbolID) :Option%200 "/SymbolRecognizerPlugin/Resources/TestContent/Textures/T_S1.T_S1" :Option%201 "/SymbolRecognizerPlugin/Resources/TestContent/Textures/T_S2.T_S2" :Option%202 "/SymbolRecognizerPlugin/Resources/TestContent/Textures/T_S3.T_S3" :Option%203 "/SymbolRecognizerPlugin/Resources/TestContent/Textures/T_S4.T_S4" :Option%204 "/SymbolRecognizerPlugin/Resources/TestContent/Textures/T_S5.T_S5" :Option%205 "/SymbolRecognizerPlugin/Resources/TestContent/Textures/T_S7.T_S7" :Option%206 "/SymbolRecognizerPlugin/Resources/TestContent/Textures/T_S8.T_S8" :Option%207 "/SymbolRecognizerPlugin/Resources/TestContent/Textures/T_S9.T_S9" :Option%208 "/SymbolRecognizerPlugin/Resources/TestContent/Textures/T_S10.T_S10" :Option%209 "/SymbolRecognizerPlugin/Resources/TestContent/Textures/T_S11.T_S11" :Option%2010 "/SymbolRecognizerPlugin/Resources/TestContent/Textures/T_S12.T_S12"))))

(event EventBeginPlay)

(event Collision|EventActorBeginOverlap
  (params (OtherActor :type Actor%20Object%20Reference)))

(fn ConstructionScript)