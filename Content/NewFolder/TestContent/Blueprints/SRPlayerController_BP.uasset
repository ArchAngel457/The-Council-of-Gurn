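; Player controller for a symbol-recognition spellcasting game that creates the HUD and switches its casting, falling-symbol and mesh-drawing menus as area events fire.
; Holding Z opens the casting panel, blocks look input and activates the pawn's magic wand, which follows the deprojected mouse.
; Left mouse opens a tick gate feeding mouse positions to the symbol recognizer.
; On release in casting mode, the best-matching symbol goes to the pawn's CastSpell.
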(event Custom|CastSpell
  (if (Default|IsCastingPanelActive (Variables|Default|GetSRHUDW))
    (bind _assrdefault_pawn_bp (Utilities|Casting|CastToSRDefaultPawn_BP (Pawn|GetControlledPawn)))
    (Default|CastSpell _assrdefault_pawn_bp (Class|SymbolRecognizer|GetMostAccurateSymbol (Class|SymbolRecognizer|GetSymbolRecognizerInstance) 0.3))))

(event Custom|EnteredDrawingMeshArea
  (Default|OpenMeshDrawingMenu (Variables|Default|GetSRHUDW)))

(event Custom|LeftDrawingMeshArea
  (Default|OpenCastingMenu (Variables|Default|GetSRHUDW)))

(event Custom|EnteredFallingSymbolArea
  (Default|OpenFallingSymbolsMenu (Variables|Default|GetSRHUDW))
  (CallFunction|ActivateWand))

(event Custom|LeftFallingSymbolArea
  (bind _srhudw (Variables|Default|GetSRHUDW))
  (Default|OpenCastingMenu _srhudw)
  (if (not (Default|IsCastingPanelActive _srhudw))
    (CallFunction|DeactivateWand)))

(event Custom|ActivateWand
  (bind (_sizex _sizey) (HUD|GetViewportSize))
  ;[1 1 1] Enable/Disable Wand
  (Components|Activation|Activate (CallFunction|GetMagicWand) false)
  (Class|PlayerController|SetMouseLocation (/ _sizex 2) (/ _sizey 2)))

(event Custom|DeactivateWand
  (bind _wand (CallFunction|GetMagicWand))
  ;[1 1 1] Enable/Disable Wand
  (if (Components|Activation|IsActive _wand)
    (Components|Activation|Deactivate _wand)))

(event EventBeginPlay
  ;[1 1 1] Create HUD
  (bind _returnvalue (UserInterface|CreateWidget "/SymbolRecognizerPlugin/Resources/TestContent/Blueprints/SRHUDWidget.SRHUDWidget_C" self))
  (bind _output_get (Variables|Default|SetSRHUDW _returnvalue))
  (UserInterface|Viewport|AddtoViewport _output_get 0))

(event EventTick
  (params (DeltaSeconds :type Float%20%28single-precision%29))
  (bind (_worldlocation _worlddirection) (Game|Player|ConvertMouseLocationToWorldSpace))
  (bind (_locationx _locationy) (Game|Player|GetMousePosition))
  (bind _srhudw (Variables|Default|GetSRHUDW))
  (Utilities|FlowControl|Sequence
    (:then_0
      ;[1 0.8275 0.3664] Draw to canvas
      (Utilities|FlowControl|Gate true
        (:Exit
          (Class|SymbolRecognizer|Draw (Class|SymbolRecognizer|GetSymbolRecognizerInstance) (Math|Vector2D|MakeVector2D _locationx _locationy)))))
    (:then_1
      ;[1 1 1] Move Magic Wand
      (if (or (Default|IsCastingPanelActive _srhudw) (Default|IsFallingSymbolsMenu _srhudw))
        (Transformation|SetWorldLocation (CallFunction|GetMagicWand) (+ _worldlocation (* _worlddirection 2e+01)) false false)))))

(event Input|KeyboardEvents|Z
  (params (Key :type Key%20Structure :default "None"))
  (bind _srhudw (Variables|Default|GetSRHUDW))
  (bind _result (Default|IsCastingMenu _srhudw))
  ;[1 1 1] Show/Hide casting panel
  (:Pressed
    (Input|SetIgnoreLookInput true)
    (if _result
      (Default|OpenCastingPanel _srhudw)
      (CallFunction|ActivateWand)))
  (:Released
    (Input|SetIgnoreLookInput false)
    (if (not (Default|IsFallingSymbolsMenu _srhudw))
      (CallFunction|DeactivateWand)
      (if _result
        (Default|HideCastingPanel _srhudw)))))

(event Input|MouseEvents|LeftMouseButton
  (params (Key :type Key%20Structure :default "None"))
  (bind (_locationx _locationy) (Game|Player|GetMousePosition))
  (bind _returnvalue (Class|SymbolRecognizer|GetSymbolRecognizerInstance))
  (bind _srhudw (Variables|Default|GetSRHUDW))
  (:Pressed
    (if (or (Default|IsCastingPanelActive _srhudw) (Default|IsFallingSymbolsMenu _srhudw))
      (CallFunction|WandResetTrail)
      ;[1 0.8275 0.3664] Draw to canvas
      (Class|SymbolRecognizer|BeginDrawing _returnvalue)
      (Utilities|FlowControl|Gate true) ; enters at Open
    ))
  (:Released
    (if (Default|IsCastingMenu _srhudw)
      (CallFunction|CastSpell)
      (Class|SymbolRecognizer|ClearCanvas (Class|SymbolRecognizer|GetSymbolRecognizerInstance))
      (Utilities|FlowControl|Sequence
        (:then_0
          (Class|SymbolRecognizer|EndDrawing _returnvalue :!label _label)
          (Utilities|FlowControl|Gate true) ; enters at Close
        )
        (:then_1
          (CallFunction|WandStopTrail :!label _label_2)
          (if (Default|IsFallingSymbolsMenu (Variables|Default|GetSRHUDW))
            (goto _label))))
      (else
        (goto _label_2)))))

(fn ConstructionScript)

(fn GetMagicWand
  (bind _assrdefault_pawn_bp (Utilities|Casting|CastToSRDefaultPawn_BP (Pawn|GetControlledPawn))
    (:then
      (bind _wand (Default|GetMagicWand _assrdefault_pawn_bp))
      (return _wand))
    (:CastFailed
      (return 0))))

(fn WandResetTrail
  (bind _assrdefault_pawn_bp (Utilities|Casting|CastToSRDefaultPawn_BP (Pawn|GetControlledPawn)))
  (Default|ResetWandTrail _assrdefault_pawn_bp))

(fn WandStopTrail
  (bind _assrdefault_pawn_bp (Utilities|Casting|CastToSRDefaultPawn_BP (Pawn|GetControlledPawn)))
  (Default|StopWandTrail _assrdefault_pawn_bp))