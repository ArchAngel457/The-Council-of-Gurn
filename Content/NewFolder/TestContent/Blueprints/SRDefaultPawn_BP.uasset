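; SRDefaultPawn_BP is a player pawn Blueprint for wand-based spellcasting.
; Helper functions expose the PMagicWand particle component, restart its trail or stop it by zeroing SpawnCount.
; CastSpell places effects relative to the eye viewpoint, with branches for ribbon trails, electric arc, wind projectile and cube.
; The switch is fixed at 0, so SpellID is only printed and the ribbon effect always spawns.
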(event EventBeginPlay)

(event Collision|EventActorBeginOverlap
  (params (OtherActor :type Actor%20Object%20Reference)))

(event EventTick
  (params (DeltaSeconds :type Float%20%28single-precision%29)))

(fn ConstructionScript)

(fn GetMagicWand
  (return (Variables|Default|GetP_MagicWand)))

(fn ResetWandTrail
  (bind _p_magicwand (Variables|Default|GetP_MagicWand))
  (Components|Activation|Deactivate _p_magicwand)
  (Effects|Components|ParticleSystem|SetFloatParameter _p_magicwand "SpawnCount" 1e+02)
  (Components|Activation|Activate _p_magicwand false))

(fn StopWandTrail
  (Effects|Components|ParticleSystem|SetFloatParameter (Variables|Default|GetP_MagicWand) "SpawnCount" 0.0))

(fn CastSpell
  (params (SpellID :type Integer))
  (bind (_outlocation _outrotation) (Actor|GetActorEyesViewPoint))
  (bind _returnvalue (Math|Vector|GetRightVector _outrotation))
  (bind _returnvalue_2 (Math|Vector|GetForwardVector _outrotation))
  (bind _returnvalue_3 (* _returnvalue 2e+01))
  (bind _returnvalue_4 (* _returnvalue_2 1e+01))
  (bind _returnvalue_5 (+ _outlocation _returnvalue_4 _returnvalue_3))
  (Development|PrintString (Utilities|String|ToString(Integer) SpellID))
  (switch int 0
    (:0
      (Effects|SpawnEmitteratLocation "/SymbolRecognizerPlugin/Resources/TestContent/Assets/P_Ribbon_trails.P_Ribbon_trails" _returnvalue_5 _outrotation))
    (:1
      (Effects|SpawnEmitteratLocation "/SymbolRecognizerPlugin/Resources/TestContent/Assets/P_electricity_arc.P_electricity_arc" _returnvalue_5 (Math|Rotator|FindLookatRotation _returnvalue_5 (+ _outlocation (* _returnvalue_2 5e+02)))))
    (:2
      (Game|SpawnActorfromClass "/Game/UI/SpellCasting/SpellCastProjectiles/Wind/SpellCast_Projectile_WindEffect.SpellCast_Projectile_WindEffect_C" (Math|Transform|MakeTransform _returnvalue_5 _outrotation "1,1,1") "AdjustIfPossibleButAlwaysSpawn" 0 0))
    (:3
      (Game|SpawnActorfromClass "/SymbolRecognizerPlugin/Resources/TestContent/Blueprints/SRCubeBP.SRCubeBP_C" (Math|Transform|MakeTransform (+ _outlocation (* _returnvalue_2 3e+02) "0,0,100.000000") "0, 0, 0" "1,1,1") "AdjustIfPossibleButAlwaysSpawn" 0 0))))