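; Falling-cubes area for the Symbol Recognizer plugin's test content, where drawn symbols are matched against falling, rotating cubes.
; Pawn overlap with ActivationBox toggles input, Tick movement and a looping spawn timer, and notifies the player controller.
; The timer recycles cubes no longer overlapping the actor, spawning when none are free, and places them atop RangeBox with random symbols.
; Mouse release sets cubes matching the recognized symbol to -1, then clears the canvas.
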(event OnComponentBeginOverlap(ActivationBox)
  (params (OverlappedComponent :type Primitive%20Component%20Object%20Reference) (OtherActor :type Actor%20Object%20Reference) (OtherComp :type Primitive%20Component%20Object%20Reference) (OtherBodyIndex :type Integer) (bFromSweep :type Boolean) (SweepResult :type Hit%20Result%20Structure%20%28by%20ref%29))
  (bind _self self)
  (bind _assrdefault_pawn_bp (Utilities|Casting|CastToSRDefaultPawn_BP OtherActor))
  (bind _assrplayer_controller_bp (Utilities|Casting|CastToSRPlayerController_BP (Pawn|GetController _assrdefault_pawn_bp)))
  (Default|EnteredFallingSymbolArea _assrplayer_controller_bp)
  (Input|EnableInput _assrplayer_controller_bp)
  (Actor|Tick|SetActorTickEnabled true)
  (if (Class|KismetSystemLibrary|IsTimerPaused _self "AddCube")
    (Class|KismetSystemLibrary|UnPauseTimer _self "AddCube")
    (else
      (Utilities|Time|SetTimerbyFunctionName _self "AddCube" 2.5 true))))

(event OnComponentEndOverlap(ActivationBox)
  (params (OverlappedComponent :type Primitive%20Component%20Object%20Reference) (OtherActor :type Actor%20Object%20Reference) (OtherComp :type Primitive%20Component%20Object%20Reference) (OtherBodyIndex :type Integer))
  (bind _assrdefault_pawn_bp (Utilities|Casting|CastToSRDefaultPawn_BP OtherActor))
  (bind _assrplayer_controller_bp (Utilities|Casting|CastToSRPlayerController_BP (Pawn|GetController _assrdefault_pawn_bp)))
  (Default|LeftFallingSymbolArea _assrplayer_controller_bp)
  (Input|DisableInput _assrplayer_controller_bp)
  (Actor|Tick|SetActorTickEnabled false)
  (Class|KismetSystemLibrary|PauseTimer self "AddCube"))

(event Custom|AddCube
  (CallFunction|SpawnorResetCube))

(event Custom|ProcessFoundSymbol
  (params (SymbolId :type Integer))
  (for _array_element (Variables|Default|GetCubes)
    (if (== SymbolId (Variables|/SymbolRecognizerPlugin/Resources/TestContent/Blueprints/SRCubeBP.SRCubeBP_C|GetSymbolID _array_element))
      (Default|SetSymbol _array_element -1))))

(event EventBeginPlay
  (Input|DisableInput (Game|GetPlayerController 0)))

(event Collision|EventActorBeginOverlap
  (params (OtherActor :type Actor%20Object%20Reference)))

(event EventTick
  (params (DeltaSeconds :type Float%20%28single-precision%29))
  (for _array_element (Variables|Default|GetCubes)
    (Transformation|AddActorLocalRotation _array_element (Math|Rotator|MakeRotator 0.0 0.0 (* DeltaSeconds 1e+01)) false false)
    (Transformation|AddActorLocalOffset _array_element (Math|Vector|MakeVector 0.0 0.0 (* DeltaSeconds -1.2e+02)) false false)))

(event Collision|EventActorEndOverlap
  (params (OtherActor :type Actor%20Object%20Reference)))

(event Input|MouseEvents|LeftMouseButton
  (params (Key :type Key%20Structure))
  (bind _returnvalue (Class|SymbolRecognizer|GetSymbolRecognizerInstance))
  (:Released
    (CallFunction|ProcessFoundSymbol (Class|SymbolRecognizer|GetMostAccurateSymbol _returnvalue 0.3))
    (Class|SymbolRecognizer|ClearCanvas _returnvalue)))

(fn ConstructionScript)

(fn SpawnorResetCube
  (bind _array_element (Utilities|Array|ForEachLoopwithBreak (Variables|Default|GetCubes) :!label _label)
    (:LoopBody
      (if (not (Collision|IsOverlappingActor _array_element self :!class /Script/Engine.Actor))
        (LocalVariables|SetLocalCube _array_element)
        (goto _label Break)))
    (:Completed
      (Utilities|IsValid (LocalVariables|GetLocalCube) :!label _label_2
        (:Is%20Valid
          (CallFunction|ResetCube (LocalVariables|GetLocalCube)))
        (:Is%20Not%20Valid
          (bind _returnvalue (Game|SpawnActorfromClass "/SymbolRecognizerPlugin/Resources/TestContent/Blueprints/SRCubeBP.SRCubeBP_C" (Math|Transform|MakeTransform "0, 0,5000.000000" "0, 0, 0" "1,1,1") "AdjustIfPossibleButAlwaysSpawn" 0 0))
          (bind _output_get (LocalVariables|SetLocalCube _returnvalue))
          (Physics|SetSimulatePhysics (Variables|/SymbolRecognizerPlugin/Resources/TestContent/Blueprints/SRCubeBP.SRCubeBP_C|GetStaticMesh _output_get) false)
          (Utilities|Array|Add (Variables|Default|GetCubes) _output_get)
          (goto _label_2))))))

(fn ResetCube
  (params (Cube :type SR%20Cube%20BP%20Object%20Reference))
  (bind _rangebox (Variables|Default|GetRangeBox))
  (bind _returnvalue (Components|Box|GetScaledBoxExtent _rangebox))
  (Transformation|SetActorLocation Cube (+ (Transformation|GetWorldLocation _rangebox) (Math|Vector|MakeVector (Math|Random|RandomFloatinRange (* (.x _returnvalue) -1.0) (.x _returnvalue)) (Math|Random|RandomFloatinRange (* (.y _returnvalue) -1.0) (.y _returnvalue)) (.z _returnvalue))) false false)
  (Default|SetSymbol Cube (Math|Random|RandomIntegerinRange 0 (- (Variables|Default|GetSymbolsCount) 1))))