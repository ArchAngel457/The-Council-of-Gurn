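; NPC_AI is the AI controller for patrolling NPCs that can detect the player.
; On BeginPlay it runs NPC_BT and seeds the blackboard with the pawn's patrol path looping, direction and wait time.
; Target perception updates write whether the player is sensed to CanSeePlayer.
; A second perception handler scans stimuli for a Noise tag but takes no action yet.
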(event OnPerceptionUpdated(AIPerception)
  (params (UpdatedActors :type Array%20of%20Actor%20Object%20References))
  (for _array_element UpdatedActors
    (bind _info (Class|AIPerceptionComponent|GetActorsPerception (Variables|Default|GetAIPerception) _array_element))
    (for _array_element_2 (.lastsensedstimuli _info)
      (if (Utilities|Name|Equal(Name) (.Tag (Utilities|Struct|BreakAIStimulus _array_element_2)) "Noise")
        _))))

(event OnTargetPerceptionUpdated(AIPerception)
  (params (Actor :type Actor%20Object%20Reference) (Stimulus :type AI%20Stimulus%20Structure))
  ;[1 1 1] AISightPerception
  (Utilities|Casting|CastToPlayerCharacter Actor)
  (AI|Components|Blackboard|SetValueasBool (AI|GetBlackboard 0) (Utilities|Name|MakeLiteralName "CanSeePlayer") (.bSuccessfullySensed (Utilities|Struct|BreakAIStimulus Stimulus))))

(event EventBeginPlay
  (bind _returnvalue (AI|GetBlackboard 0))
  (AI|RunBehaviorTree "/Game/AI/NPC/NPC_BT.NPC_BT")
  (bind _asnpc (Utilities|Casting|CastToNPC (Pawn|GetControlledPawn)))
  (bind _output_get (Variables|Default|SetMyPawn _asnpc))
  (AI|Components|Blackboard|SetValueasBool (AI|GetBlackboard 0) (Utilities|Name|MakeLiteralName "PathLooping") (Variables|/Game/AI/NPC/Blueprints/PatrolPath.PatrolPath_C|GetIsLooping (Variables|/Game/AI/NPC/Blueprints/NPC.NPC_C|GetPatrolPath _output_get)))
  (Class|BlackboardComponent|SetValueasInt _returnvalue (Utilities|Name|MakeLiteralName "Direction") 1)
  (AI|Components|Blackboard|SetValueasFloat _returnvalue (Utilities|Name|MakeLiteralName "WaitTime") (Variables|/Game/AI/NPC/Blueprints/PatrolPath.PatrolPath_C|GetWaitTime (Variables|/Game/AI/NPC/Blueprints/NPC.NPC_C|GetPatrolPath (Variables|Default|GetMyPawn)))))

(fn ConstructionScript)