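; NPC Blueprint for an AI character that can play a melee attack and be knocked into a ragdoll.
; The MeleeAttack event plays the primary attack montage on the mesh.
; The Force event waits briefly, switches the mesh to simulated ragdoll physics and launches it with a large impulse along the player's control-rotation forward vector.
; It then disables capsule collision, provided the PlayerCharacter cast succeeds.
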(event Custom|Force
  ;[1 1 1] ForceNPC
  (Utilities|FlowControl|Delay 0.5)
  (Collision|SetCollisionProfileName (Variables|Character|GetMesh) "Ragdoll" :!class /Script/Engine.PrimitiveComponent)
  (Physics|SetSimulatePhysics (Variables|Character|GetMesh) true)
  (bind _asplayer_character (Utilities|Casting|CastToPlayerCharacter (Game|GetPlayerCharacter 0)))
  (Physics|AddImpulse (Variables|Character|GetMesh) (* (Math|Vector|GetForwardVector (Pawn|GetControlRotation _asplayer_character :!class /Script/Engine.Pawn)) 3e+05) "None" false)
  (Collision|SetCollisionEnabled (Variables|Collision|GetCapsuleComponent) "NoCollision"))

(event EventMeleeAttack
  (Animation|Montage|PlayMontage (Variables|Character|GetMesh) "/Game/FORTESTONLY/Mannequin/Animations/Attack_PrimaryA_Montage.Attack_PrimaryA_Montage"))

(fn ConstructionScript)